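; BP_C1JoyKit is an interactable joy kit object in Part 1 that the player picks up to start a fight sequence.
; On Interact it runs the parent logic, disables further interaction and hides itself in game.
; It then reveals the JoyKit component on the player's VRPawn and calls StartFightAfterJoyKit on the level's BP_Part1Manager.
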(fn `Interact`
  (`parent.Interact`)
  (set `self.CanInteract` false)
  (`self.SetActorHiddenInGame` true)
  (bind _asvrpawn (cast `/Game/VRTemplate/Blueprints/VRPawn` (`GameplayStatics.GetPlayerPawn` 0)))
  (bind _joykit (`/Game/VRTemplate/Blueprints/VRPawn.JoyKit` _asvrpawn))
  (`SceneComponent.SetVisibility` _joykit true false)
  (`SceneComponent.SetHiddenInGame` _joykit false false)
  (bind _outactors (`GameplayStatics.GetAllActorsOfClass` "/Game/00_MY/03_BP/BP_Part1Manager.BP_Part1Manager_C"))
  (`/Game/00_MY/03_BP/BP_Part1Manager.StartFightAfterJoyKit` (`|GetArrayItem` _outactors)))

(fn `UserConstructionScript`)