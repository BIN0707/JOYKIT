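; BP_DrawingPencil is a pencil actor that shows a simple drawing motion on demand, hidden in game until triggered.
; It caches its starting transform on BeginPlay, then StartDrawingPencil reveals PenAni and plays a timeline that lerps the actor along a small diagonal XY offset.
; StopDrawingPencil halts the timeline, restores the cached location and rotation, and hides PenAni again.
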(event `self.ReceiveBeginPlay`
  (set `self.StartLocation` (`self.K2_GetActorLocation`))
  (set `self.StartRotation` (`self.K2_GetActorRotation`))
  (`SceneComponent.SetHiddenInGame` (`self.Pen_Ani`) true false))

(event `StartDrawingPencil`
  (`SceneComponent.SetHiddenInGame` (`self.Pen_Ani`) false false)
  (bind (_direction _movealpha) (`Timeline|TL_PencilDraw` :!label _label)
    (:`Update`
      (`self.K2_SetActorLocation` (`KismetMathLibrary.VLerp` (`self.StartLocation`) (+ (`self.StartLocation`) (5.0 5.0 0.0)) _movealpha)))))

(event `StopDrawingPencil`
  (`|ExecutionSequence`
    (:`then_0`
      (goto _label :!via `Stop`))
    (:`then_1`
      (`self.K2_SetActorLocation` (`self.StartLocation`))
      (`self.K2_SetActorRotation` (`self.StartRotation`))
      (`SceneComponent.SetHiddenInGame` (`self.Pen_Ani`) true false))))

(fn `UserConstructionScript`)