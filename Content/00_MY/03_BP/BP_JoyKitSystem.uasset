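; JoyKit system that tracks player anxiety and shows it through post-process visuals.
; Anxiety changes set target weights for Default, Stable and Anxious post-process states, with a timeline meant to crossfade them.
; Crossing the threshold opens a choice UI on VRPawn; Stable zeroes anxiety and switches state, Endure keeps it, and each fires its event.
; A recovery timeline eases anxiety back to baseline without re-triggering the choice.
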(event `UpdateAnxietyPP`
  (set `self.AnxietyAlpha` (`KismetMathLibrary.FClamp` (/ (- (`self.Anxiety`) (`self.BaseAnxiety`)) (- (`self.MaxAnxiety`) (`self.BaseAnxiety`)))))
  (set `self.StartDefaultWeight` (`self.CurrentDefaultWeight`))
  (set `self.StartStableWeight` (`self.CurrentStableWeight`))
  (set `self.StartAnxiousWeight` (`self.CurrentAnxiousWeight`))
  (set `self.TargetDefaultWeight` (- 1.0 (`self.AnxietyAlpha`)))
  (set `self.TargetStableWeight` 0.0)
  (set `self.TargetAnxiousWeight` (`self.AnxietyAlpha`))
  (`TimelineComponent.PlayFromStart` (`self.TL_PPTransition`)))

(event `SetAnxiety`
  (params (NewValue :type "Float (double-precision)"))
  (set `self.Anxiety` (`KismetMathLibrary.FClamp` NewValue (`self.BaseAnxiety`) (`self.MaxAnxiety`)))
  (`self.UpdateAnxietyPP`)
  (`self.CheckThreshold`))

(event `SetAnxietyNoThreshold`
  (params (Value :type "Float (double-precision)"))
  (set `self.Anxiety` (`KismetMathLibrary.FClamp` Value 0.0 (`self.MaxAnxiety`)))
  (`self.UpdateAnxietyPP`))

(event `ReturnToDefaultGradually`
  (set `self.RecoveryStartAnxiety` (`self.Anxiety`))
  (set `self.RecoveryTargetAnxiety` (`self.BaseAnxiety`))
  (`self.SetState_Default`)
  (bind (_direction _alpha) (`Timeline|TL_AnxietyRecovery` :!via `PlayFromStart`)
    (:`Update`
      (`self.SetAnxietyNoThreshold` (`KismetMathLibrary.Lerp` (`self.RecoveryStartAnxiety`) (`self.RecoveryTargetAnxiety`) _alpha)))
    (:`Finished`
      (`KismetSystemLibrary.PrintString` "평상 상태 복귀"))))

(event `CheckThreshold`
  (if (and (>= (`self.Anxiety`) (`self.Threshold`)) (not (`self.bChoiceShown`)))
    (set `self.bChoiceShown` true)
    (bind _asvrpawn (cast `/Game/VRTemplate/Blueprints/VRPawn` (`GameplayStatics.GetPlayerPawn` 0)))
    (`/Game/VRTemplate/Blueprints/VRPawn.OpenChoiceUI` _asvrpawn)))

(event `SelectStable`
  (set `self.Anxiety` 0.0)
  (bind _asvrpawn (cast `/Game/VRTemplate/Blueprints/VRPawn` (`GameplayStatics.GetPlayerPawn` 0)))
  (`/Game/VRTemplate/Blueprints/VRPawn.CloseChoiceUI` _asvrpawn)
  (set `self.bChoiceShown` false)
  (`self.SetState_Stable`)
  (`self.OnStableSelected`))

(event `SelectEndure`
  (bind _asvrpawn (cast `/Game/VRTemplate/Blueprints/VRPawn` (`GameplayStatics.GetPlayerPawn` 0)))
  (`/Game/VRTemplate/Blueprints/VRPawn.CloseChoiceUI` _asvrpawn)
  (set `self.bChoiceShown` false)
  (`self.OnEndureSelected`))

(event `SetState_Default`
  (set `self.StartDefaultWeight` (`self.CurrentDefaultWeight`))
  (set `self.StartStableWeight` (`self.CurrentStableWeight`))
  (set `self.StartAnxiousWeight` (`self.CurrentAnxiousWeight`))
  (set `self.TargetDefaultWeight` 1.0)
  (set `self.TargetStableWeight` 0.0)
  (set `self.TargetAnxiousWeight` 0.0)
  (`TimelineComponent.PlayFromStart` (`self.TL_PPTransition`)))

(event `SetState_Stable`
  (set `self.StartDefaultWeight` (`self.CurrentDefaultWeight`))
  (set `self.StartStableWeight` (`self.CurrentStableWeight`))
  (set `self.StartAnxiousWeight` (`self.CurrentAnxiousWeight`))
  (set `self.TargetDefaultWeight` 0.0)
  (set `self.TargetStableWeight` 1.0)
  (set `self.TargetAnxiousWeight` 0.0)
  (`TimelineComponent.PlayFromStart` (`self.TL_PPTransition`)))

(event `SetState_Anxious`
  (set `self.StartDefaultWeight` (`self.CurrentDefaultWeight`))
  (set `self.StartStableWeight` (`self.CurrentStableWeight`))
  (set `self.StartAnxiousWeight` (`self.CurrentAnxiousWeight`))
  (set `self.TargetDefaultWeight` 0.0)
  (set `self.TargetStableWeight` 0.0)
  (set `self.TargetAnxiousWeight` 1.0)
  (`TimelineComponent.PlayFromStart` (`self.TL_PPTransition`)))

(fn `UserConstructionScript`)