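; Scene director for Part 1 of a VR story where a child draws a family-picture homework while parents argue nearby.
; Delay-timed events sync VR subtitles, voices, TV audio and sketchbook drawing, raising JoyKit anxiety as the fight escalates.
; JoyKit stable/endure delegates branch the dialogue and drawing, then both paths ease anxiety and end the part.
; It also starts the desk sequence, enables JoyKit interactions and counts investigations to unlock the desk.
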(event `PlayParentDialogueSound`
  (params (SoundIndex :type Integer) (Volume :type "Float (double-precision)"))
  (`GameplayStatics.PlaySoundAtLocation` (`|GetArrayItem` (`self.ParentDialogueSounds`) SoundIndex) (`self.K2_GetActorLocation` (`self.ParentVoicePoint`)) (struct) Volume 1.0 0.0 null null null null))

(event `PlayChildDialogueSound`
  (params (`Sound Index` :type Integer) (Volume :type "Float (double-precision)"))
  (`GameplayStatics.PlaySound2D` (`|GetArrayItem` (`self.ChildDialogueSounds`) `Sound Index`) Volume 1.0 0.0 null null))

(event `StartJoyKitBoxInspect`
  ; 조이키트 박스 상호작용 이후 대사
  (`KismetSystemLibrary.Delay` 0.7)
  (`self.ShowDialogue` "불안을 줄여주는 장치? … 언제 여기 있었지.")
  (`self.PlayChildDialogueSound` 3 2.0)
  (`KismetSystemLibrary.Delay` 3.0)
  (`self.HideDialogue`)
  (`self.SetActorHiddenInGame` (`self.JoyKitBoxRef`) true)
  (bind _outactors (`GameplayStatics.GetAllActorsOfClass` "/Game/00_MY/03_BP/Part01_Object/BP_C1JoyKit.BP_C1JoyKit_C"))
  (bind _output (`|GetArrayItem` _outactors))
  (`self.SetActorHiddenInGame` _output false)
  (set `/Game/00_MY/03_BP/BP_InteractObject.CanInteract` true _output)
  (`/Game/00_MY/03_BP/BP_InteractObject.UpdatePromptVisibility` _output))

(event `StartHomeworkScene`
  (bind _joykitboxref (`self.JoyKitBoxRef`))
  ; 숙제 시작 씬
  (`KismetSystemLibrary.Delay` 1.0)
  (`self.ShowDialogue` "오늘 학교에서 연락왔어.")
  (`self.PlayParentDialogueSound` 0 0.7)
  (`KismetSystemLibrary.Delay` 3.0)
  (`self.ShowDialogue` "…하. 왜 또.")
  (`self.PlayParentDialogueSound` 1 0.7)
  (`KismetSystemLibrary.Delay` 2.0)
  (`self.ShowDialogue` "애가 요즘 수업에 집중을 잘 못한대.")
  (`self.PlayParentDialogueSound` 2 0.7)
  (`KismetSystemLibrary.Delay` 3.0)
  (`self.ShowDialogue` "선생님이 애랑 따로 얘기 좀 해보라고 하셨어.")
  (`self.PlayParentDialogueSound` 3 0.7)
  (`KismetSystemLibrary.Delay` 4.0)
  (`self.ShowDialogue` "또 그 얘기네.")
  (`self.PlayParentDialogueSound` 4 0.7)
  (`KismetSystemLibrary.Delay` 1.0)
  (`self.ShowDialogue` "그래서. 나보고 뭐 어쩌라고.")
  (`self.PlayParentDialogueSound` 5 0.7)
  (`KismetSystemLibrary.Delay` 3.0)
  (bind _outactors (`GameplayStatics.GetAllActorsOfClass` "/Game/00_MY/03_BP/BP_JoyKitSystem.BP_JoyKitSystem_C"))
  (`/Game/00_MY/03_BP/BP_JoyKitSystem.SetAnxiety` (`|GetArrayItem` _outactors) 30.0)
  (`self.ShowDialogue` "같이 좀 보자고…")
  (`self.PlayParentDialogueSound` 6 0.7)
  (`KismetSystemLibrary.Delay` 1.5)
  (`self.ShowDialogue` "내가 지금 그것까지 신경 쓸 여유가 어딨어.")
  (`self.PlayParentDialogueSound` 7 0.7)
  (`KismetSystemLibrary.Delay` 3.0)
  (`self.ShowDialogue` "내가 놀고만 있냐? 일하느라 바빠!")
  (`self.PlayParentDialogueSound` 8 0.8)
  (`KismetSystemLibrary.Delay` 4.0)
  (bind _outactors_2 (`GameplayStatics.GetAllActorsOfClass` "/Game/00_MY/03_BP/BP_JoyKitSystem.BP_JoyKitSystem_C"))
  (`/Game/00_MY/03_BP/BP_JoyKitSystem.SetAnxiety` (`|GetArrayItem` _outactors_2) 40.0)
  (`self.ShowDialogue` "조용히 좀 말해..! 애 듣는다고!")
  (`self.PlayParentDialogueSound` 9 0.85)
  (`KismetSystemLibrary.Delay` 2.0)
  (`self.IncreaseTVVolume` 0.6)
  (`self.ShowDialogue` "(TV소리)")
  (`KismetSystemLibrary.Delay` 3.0)
  (`/Game/00_MY/03_BP/Part01_Object/BP_C1Sketchbook.StopSketchbookReveal` (`self.SketchbookRef`))
  (`self.StopDrawingSound`)
  (`/Game/00_MY/03_BP/BP_DrawingPencil.StopDrawingPencil` (`self.DrawingPencilRef`))
  (`self.ShowDialogue` "음…. 집중이 잘 안되네")
  (`self.PlayChildDialogueSound` 2 2.0)
  (`KismetSystemLibrary.Delay` 3.0)
  (`self.HideDialogue`)
  (set `/Game/00_MY/03_BP/BP_InteractObject.CanInteract` true _joykitboxref)
  (`/Game/00_MY/03_BP/BP_InteractObject.UpdatePromptVisibility` _joykitboxref))

(event `StartDeskUnlockedDialogue`
  (bind _deskref (`self.DeskRef`))
  (`self.ShowDialogue` "아이 : 우선 숙제부터 해야겠다.")
  (`KismetSystemLibrary.Delay` 2.0)
  (`self.HideDialogue`)
  (set `self.bDeskUnlocked` true)
  (set `/Game/00_MY/03_BP/BP_InteractObject.CanInteract` true _deskref)
  (`/Game/00_MY/03_BP/BP_InteractObject.UpdatePromptVisibility` _deskref))

(event `StartDeskScene`
  (`KismetSystemLibrary.Delay` 10.0)
  (`self.PlayTVSound` 0.25)
  (`KismetSystemLibrary.Delay` 3.0)
  (`self.ShowDialogue` "내일까지 가족 그림 그리기 숙제가 있었지")
  (`self.PlayChildDialogueSound` 0 2.0)
  (`KismetSystemLibrary.Delay` 3.0)
  (`self.ShowDialogue` "우선 숙제부터 해야겠다.")
  (`self.PlayChildDialogueSound` 1 2.0)
  (`KismetSystemLibrary.Delay` 3.0)
  (`self.HideDialogue`)
  (`KismetSystemLibrary.Delay` 5.0)
  (`self.PlayDrawingSound`)
  (`/Game/00_MY/03_BP/BP_DrawingPencil.StartDrawingPencil` (`self.DrawingPencilRef`))
  (`/Game/00_MY/03_BP/Part01_Object/BP_C1Sketchbook.RevealSketchbookTexture` (`self.SketchbookRef`) "/Game/00_MY/04_Texture/Part1/Sketchbook/Sketchbook_Draft_T.Sketchbook_Draft_T" 1.0)
  (`self.StartHomeworkScene`))

(event `PlayTVSound`
  (params (Volume :type "Float (double-precision)"))
  ; TV 사운드
  (bind _returnvalue (`GameplayStatics.SpawnSoundAtLocation` (`self.SFX_TV`) (`self.K2_GetActorLocation` (`self.ParentVoicePoint`)) (struct) Volume 1.0 0.0 null null))
  (set `self.TVAudioComponent` _returnvalue))

(event `StopTVSound`
  ; TV 사운드
  (`AudioComponent.FadeOut` (`self.TVAudioComponent`) 5.0 0.0 "Linear"))

(event `StartFightAfterJoyKit`
  ; 조이키트 착용 후 싸움
  (`KismetSystemLibrary.Delay` 2.0)
  (`self.ShowDialogue` "그래서")
  (`self.PlayParentDialogueSound` 10 1.0)
  (`KismetSystemLibrary.Delay` 1.0)
  (`self.ShowDialogue` "지금 애 문제까지 다 내 탓이라는 거야?")
  (`self.PlayParentDialogueSound` 11 1.0)
  (`KismetSystemLibrary.Delay` 3.0)
  (bind _outactors (`GameplayStatics.GetAllActorsOfClass` "/Game/00_MY/03_BP/BP_JoyKitSystem.BP_JoyKitSystem_C"))
  (`/Game/00_MY/03_BP/BP_JoyKitSystem.SetAnxiety` (`|GetArrayItem` _outactors) 60.0)
  (`self.ShowDialogue` "탓이 아니라… 얘기 좀 하자는 거잖아…")
  (`self.PlayParentDialogueSound` 12 1.0)
  (`KismetSystemLibrary.Delay` 3.0)
  (`self.ShowDialogue` "맨날 똑같은 소리!")
  (`self.PlayParentDialogueSound` 13 1.0)
  (`KismetSystemLibrary.Delay` 2.0)
  (`self.ShowDialogue` "하 지겹지도 않아?")
  (`self.PlayParentDialogueSound` 14 1.0)
  (`KismetSystemLibrary.Delay` 2.0)
  (bind _outactors_2 (`GameplayStatics.GetAllActorsOfClass` "/Game/00_MY/03_BP/BP_JoyKitSystem.BP_JoyKitSystem_C"))
  (`/Game/00_MY/03_BP/BP_JoyKitSystem.SetAnxiety` (`|GetArrayItem` _outactors_2) 70.0)
  (`self.ShowDialogue` "그럼 말하는거 한 번이라도 들어준 적 있어?")
  (`self.PlayParentDialogueSound` 15 1.0)
  (`KismetSystemLibrary.Delay` 4.0)
  (`self.ShowDialogue` "나도 똑같은 소리 맨날 하는거 지겨워!")
  (`self.PlayParentDialogueSound` 16 1.0)
  (`KismetSystemLibrary.Delay` 3.0)
  (`self.ShowDialogue` "뭐? 어디서 소리를 질러!!")
  (`self.PlayParentDialogueSound` 17 1.0)
  (`KismetSystemLibrary.Delay` 3.0)
  (`self.HideDialogue`)
  (`KismetSystemLibrary.PrintString` "유리 깨지는 소리")
  (bind _outactors_3 (`GameplayStatics.GetAllActorsOfClass` "/Game/00_MY/03_BP/BP_JoyKitSystem.BP_JoyKitSystem_C"))
  (`/Game/00_MY/03_BP/BP_JoyKitSystem.SetAnxiety` (`|GetArrayItem` _outactors_3) 80.0))

(event `IncreaseTVVolume`
  (params (NewVolume :type "Float (double-precision)"))
  ; TV 사운드
  (`AudioComponent.SetVolumeMultiplier` (`self.TVAudioComponent`) NewVolume))

(event `PlayDrawingSound`
  (bind _returnvalue (`GameplayStatics.SpawnSound2D` (`self.SFX_DrawingLoop`) 1.0 1.0 0.0 null))
  (set `self.DrawingAudioComponent` _returnvalue))

(event `StopDrawingSound`
  (bind _drawingaudiocomponent (`self.DrawingAudioComponent`))
  (`/Engine/EditorBlueprintResources/StandardMacros.IsValid` _drawingaudiocomponent
    (:`Is Valid`
      (`AudioComponent.FadeOut` _drawingaudiocomponent 0.5 0.0 "Linear")
      (set `self.DrawingAudioComponent` null))))

(event `Part1_End`
  (`KismetSystemLibrary.PrintString` "파트1 종료"))

(event `ShowDialogue`
  (params (DialogueText :type Text))
  (`/Game/VRTemplate/Blueprints/VRPawn.ShowDialogueVR` (`self.VRPawnRef`) DialogueText))

(event `self.ReceiveBeginPlay`
  (bind _outactors (`GameplayStatics.GetAllActorsOfClass` "/Game/00_MY/03_BP/BP_JoyKitSystem.BP_JoyKitSystem_C"))
  (bind _output (`|GetArrayItem` _outactors))
  (add `/Game/00_MY/03_BP/BP_JoyKitSystem.OnStableSelected` _output (delegate `Part1_StartStableAfterChoice`))
  (add `/Game/00_MY/03_BP/BP_JoyKitSystem.OnEndureSelected` _output (delegate `Part1_StartEndureAfterChoice`))
  (bind _asvrpawn (cast `/Game/VRTemplate/Blueprints/VRPawn` (`GameplayStatics.GetPlayerPawn` 0)))
  (set `self.VRPawnRef` _asvrpawn)
  (bind _outactors_2 (`GameplayStatics.GetAllActorsOfClass` "/Game/00_MY/03_BP/Part01_Object/BP_C1Desk.BP_C1Desk_C"))
  (`/Game/00_MY/03_BP/Part01_Object/BP_C1Desk.StartDeskSequence` (`|GetArrayItem` _outactors_2)))

(event `HideDialogue`
  (`/Game/VRTemplate/Blueprints/VRPawn.HideDialogueVR` (`self.VRPawnRef`)))

(event `Part1_StartStableAfterChoice`
  (set `self.Part1ChoiceResult` 1)
  (`KismetSystemLibrary.Delay` 2.0)
  (`self.ShowDialogue` "밥은 먹었어?")
  (`self.PlayParentDialogueSound` 22 1.0)
  (`KismetSystemLibrary.Delay` 1.5)
  (`self.ShowDialogue` "아직. 안 먹고 바로 집으로 왔지.")
  (`self.PlayParentDialogueSound` 23 1.0)
  (`KismetSystemLibrary.Delay` 3.0)
  (`self.PlayDrawingSound`)
  (`/Game/00_MY/03_BP/BP_DrawingPencil.StartDrawingPencil` (`self.DrawingPencilRef`))
  (`/Game/00_MY/03_BP/Part01_Object/BP_C1Sketchbook.RevealSketchbookTexture` (`self.SketchbookRef`) "/Game/00_MY/04_Texture/Part1/Sketchbook/Sketchbook_Stable_T.Sketchbook_Stable_T" 0.5)
  (`self.ShowDialogue` "많이 힘들겠다. 오늘은 좀 늦게 왔네")
  (`self.PlayParentDialogueSound` 24 1.0)
  (`KismetSystemLibrary.Delay` 2.0)
  (`self.PlayParentDialogueSound` 25 1.0)
  (`KismetSystemLibrary.Delay` 2.0)
  (`self.ShowDialogue` "금방 밥 차려줄게.")
  (`self.PlayParentDialogueSound` 26 1.0)
  (`KismetSystemLibrary.Delay` 2.0)
  (`self.ShowDialogue` "괜찮아. 천천히 해.")
  (`self.PlayParentDialogueSound` 27 1.0)
  (`KismetSystemLibrary.Delay` 1.0)
  (`self.PlayParentDialogueSound` 28 1.0)
  (`KismetSystemLibrary.Delay` 2.0)
  (`self.HideDialogue`)
  (`KismetSystemLibrary.Delay` 3.0)
  (`self.ShowDialogue` "음.. 아까? 괜찮은건가?")
  (`self.PlayChildDialogueSound` 5 2.0)
  (`KismetSystemLibrary.Delay` 3.0)
  (`self.HideDialogue`)
  (`KismetSystemLibrary.Delay` 1.0)
  (`self.Part1_DrawStableResult`))

(event `Part1_StartEndureAfterChoice`
  (set `self.Part1ChoiceResult` 2)
  (`KismetSystemLibrary.Delay` 2.0)
  (`self.ShowDialogue` "… 진짜 계속 이럴 거야?")
  (`self.PlayParentDialogueSound` 18 1.0)
  (`KismetSystemLibrary.Delay` 2.5)
  (`self.ShowDialogue` "그러니까 그만 좀 하라고 했지.")
  (`self.PlayParentDialogueSound` 19 1.0)
  (`KismetSystemLibrary.Delay` 3.0)
  (`self.PlayDrawingSound`)
  (`/Game/00_MY/03_BP/BP_DrawingPencil.StartDrawingPencil` (`self.DrawingPencilRef`))
  (`/Game/00_MY/03_BP/Part01_Object/BP_C1Sketchbook.RevealSketchbookTexture` (`self.SketchbookRef`) "/Game/00_MY/04_Texture/Part1/Sketchbook/Sketchbook_Anxious_T.Sketchbook_Anxious_T" 0.5)
  (`self.ShowDialogue` "적어도 애 앞에서는…")
  (`self.PlayParentDialogueSound` 20 1.0)
  (`KismetSystemLibrary.Delay` 2.0)
  (`self.ShowDialogue` "내가 알아서 해.")
  (`self.PlayParentDialogueSound` 21 1.0)
  (`KismetSystemLibrary.Delay` 2.0)
  (`self.HideDialogue`)
  (`KismetSystemLibrary.Delay` 4.0)
  (`self.ShowDialogue` "아이 : ...")
  (`KismetSystemLibrary.Delay` 1.0)
  (`self.HideDialogue`)
  (`KismetSystemLibrary.Delay` 1.0)
  (`self.Part1_DrawEndureResult`))

(event `Part1_DrawStableResult`
  (`KismetSystemLibrary.Delay` 5.0)
  (`/Game/00_MY/03_BP/Part01_Object/BP_C1Sketchbook.StopSketchbookReveal` (`self.SketchbookRef`))
  (`self.StopDrawingSound`)
  (`/Game/00_MY/03_BP/BP_DrawingPencil.StopDrawingPencil` (`self.DrawingPencilRef`))
  (`self.PlayChildDialogueSound` 6 2.0)
  (`self.ShowDialogue` "다 그렸다! 음… 괜찮나..?")
  (`KismetSystemLibrary.Delay` 3.0)
  (`self.HideDialogue`)
  (bind _outactors (`GameplayStatics.GetAllActorsOfClass` "/Game/00_MY/03_BP/BP_JoyKitSystem.BP_JoyKitSystem_C"))
  (`/Game/00_MY/03_BP/BP_JoyKitSystem.ReturnToDefaultGradually` (`|GetArrayItem` _outactors))
  (`KismetSystemLibrary.Delay` 3.0)
  (`self.ShowDialogue` "엄마: 밥 먹어.")
  (`self.PlayParentDialogueSound` 29 1.0)
  (`KismetSystemLibrary.Delay` 2.0)
  (`self.HideDialogue`)
  (`self.Part1_End`))

(event `Part1_DrawEndureResult`
  (`KismetSystemLibrary.Delay` 5.0)
  (`/Game/00_MY/03_BP/Part01_Object/BP_C1Sketchbook.StopSketchbookReveal` (`self.SketchbookRef`))
  (`self.StopDrawingSound`)
  (`/Game/00_MY/03_BP/BP_DrawingPencil.StopDrawingPencil` (`self.DrawingPencilRef`))
  (`self.PlayChildDialogueSound` 4 2.0)
  (`self.ShowDialogue` "…왜 이렇게 그려지지. 근데 이게 맞는 것 같기도 하고…")
  (`KismetSystemLibrary.Delay` 4.0)
  (`self.HideDialogue`)
  (bind _outactors (`GameplayStatics.GetAllActorsOfClass` "/Game/00_MY/03_BP/BP_JoyKitSystem.BP_JoyKitSystem_C"))
  (`/Game/00_MY/03_BP/BP_JoyKitSystem.ReturnToDefaultGradually` (`|GetArrayItem` _outactors))
  (`KismetSystemLibrary.Delay` 3.0)
  (`self.ShowDialogue` "엄마: 밥 먹어.")
  (`self.PlayParentDialogueSound` 29 1.0)
  (`KismetSystemLibrary.Delay` 2.0)
  (`self.HideDialogue`)
  (`self.Part1_End`))

(fn `AddInvestigationCount`
  (set `self.InvestigatedCount` (+ (`self.InvestigatedCount`) 1))
  (`KismetSystemLibrary.PrintString` (`KismetStringLibrary.Conv_IntToString` (`self.InvestigatedCount`)))
  (if (and (>= (`self.InvestigatedCount`) (`self.RequiredInvestigations`)) (not (`self.bDeskUnlocked`)))
    (`self.StartDeskUnlockedDialogue`)))

(fn `UserConstructionScript`)