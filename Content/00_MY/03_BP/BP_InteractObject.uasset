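; BP_InteractObject is an interactable object for the VR pawn, offering a prompt and an inspection when used.
; A range trigger shows the prompt widget while interaction is allowed, and Tick yaws it toward the camera.
; Interact hides the prompt, then opens the pawn's animated or mesh inspect, or just prints the interaction text.
; CompleteInvestigation adds to the BP_Part1Manager investigation count only once per object.
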(event `CompleteInvestigation`
  (if (not (`self.HasInteracted`))
    (set `self.HasInteracted` true)
    (bind _outactors (`GameplayStatics.GetAllActorsOfClass` "/Game/00_MY/03_BP/BP_Part1Manager.BP_Part1Manager_C"))
    (`/Game/00_MY/03_BP/BP_Part1Manager.AddInvestigationCount` (`|GetArrayItem` _outactors))))

(event `self.ReceiveTick`
  (params (DeltaSeconds :type "Float (single-precision)"))
  (if (`self.bPromptVisible`)
    (`SceneComponent.K2_SetWorldRotation` (`self.PromptWidget`) (`KismetMathLibrary.MakeRotator` 0.0 0.0 (.yaw (`KismetMathLibrary.FindLookAtRotation` (`SceneComponent.K2_GetComponentLocation` (`self.PromptWidget`)) (`PlayerCameraManager.GetCameraLocation` (`GameplayStatics.GetPlayerCameraManager` 0))))) false false)))

(event `self.PromptRange.OnComponentBeginOverlap`
  (params (OverlappedComponent :type "PrimitiveComponent Object Reference") (OtherActor :type "Actor Object Reference") (OtherComp :type "PrimitiveComponent Object Reference") (OtherBodyIndex :type Integer) (bFromSweep :type Boolean) (SweepResult :type "HitResult Structure (by ref)"))
  (cast `/Game/VRTemplate/Blueprints/VRPawn` OtherActor)
  (if (`self.CanInteract`)
    (set `self.bPromptVisible` true)
    (`SceneComponent.SetHiddenInGame` (`self.PromptWidget`) false false)))

(event `self.PromptRange.OnComponentEndOverlap`
  (params (OverlappedComponent :type "PrimitiveComponent Object Reference") (OtherActor :type "Actor Object Reference") (OtherComp :type "PrimitiveComponent Object Reference") (OtherBodyIndex :type Integer))
  (cast `/Game/VRTemplate/Blueprints/VRPawn` OtherActor)
  (set `self.bPromptVisible` false)
  (`SceneComponent.SetHiddenInGame` (`self.PromptWidget`) true false))

(fn `Interact`
  (set `self.bPromptVisible` false)
  (`SceneComponent.SetHiddenInGame` (`self.PromptWidget`) true false)
  (if (`self.CanInteract`)
    (if (`self.UseAnimatedInspect`)
      (bind _asvrpawn (cast `/Game/VRTemplate/Blueprints/VRPawn` (`GameplayStatics.GetPlayerPawn` 0)))
      (`/Game/VRTemplate/Blueprints/VRPawn.OpenAnimatedInspect` _asvrpawn self (`self.InspectText`) (`self.AnimatedInspectReadDelay`) (`self.AnimatedInspectSkeletalMesh`) (`self.AnimatedInspectAnimation`) (`self.AnimatedInspectResultMesh`))
      (elif (`self.bUseInspectMode`)
        (bind _asvrpawn_2 (cast `/Game/VRTemplate/Blueprints/VRPawn` (`GameplayStatics.GetPlayerPawn` 0)))
        (`/Game/VRTemplate/Blueprints/VRPawn.OpenInspect` _asvrpawn_2 (`self.InspectStaticMesh`) (`self.InspectMaterial`) (`self.InspectText`) self)
        (else
          (`KismetSystemLibrary.PrintString` (`KismetTextLibrary.Conv_TextToString` (`self.InteractionText`))))))))

(fn `UpdatePromptVisibility`
  (if (and (> (`KismetArrayLibrary.Array_Length` (`PrimitiveComponent.GetOverlappingActors` (`self.PromptRange`) "/Game/VRTemplate/Blueprints/VRPawn.VRPawn_C")) 0) (`self.CanInteract`))
    (set `self.bPromptVisible` true)
    (`SceneComponent.SetHiddenInGame` (`self.PromptWidget`) false false)
    (else
      (set `self.bPromptVisible` false)
      (`SceneComponent.SetHiddenInGame` (`self.PromptWidget`) true false))))

(fn `UserConstructionScript`)