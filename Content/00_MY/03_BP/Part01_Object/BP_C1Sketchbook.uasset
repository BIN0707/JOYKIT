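; Interactable Part 1 sketchbook that reveals a drawing matching the player's choice and advances the story.
; BeginPlay puts a dynamic reveal material on the cube, showing the default page.
; Interact disables further interaction, reads the choice result from BP_Part1Manager, picks the draft, stable or anxious texture and triggers the matching manager event.
; A rate-adjustable timeline drives RevealAmount from current to new texture, storing it as current when finished.
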(event `self.ReceiveBeginPlay`
  (bind _returnvalue (`PrimitiveComponent.CreateDynamicMaterialInstance` (`self.Cube`) 0 "/Game/00_MY/02_Material/M_Sketchbook_Reveal.M_Sketchbook_Reveal" "None"))
  (bind _output_get (set `self.MID_Sketchbook` _returnvalue))
  (set `self.CurrentTexture` (`self.Tex_Default`))
  (`MaterialInstanceDynamic.SetTextureParameterValue` _output_get "BaseTexture" (`self.Tex_Default`))
  (`MaterialInstanceDynamic.SetTextureParameterValue` _output_get "TargetTexture" (`self.Tex_Default`))
  (`MaterialInstanceDynamic.SetScalarParameterValue` _output_get "RevealAmount" 1.0))

(event `RevealSketchbookTexture`
  (params (NewTexture :type "Texture2D Object Reference") (RevealPlayRate :type "Float (double-precision)"))
  (set `self.PendingTexture` NewTexture)
  (`MaterialInstanceDynamic.SetTextureParameterValue` (`self.MID_Sketchbook`) "BaseTexture" (`self.CurrentTexture`))
  (`MaterialInstanceDynamic.SetTextureParameterValue` (`self.MID_Sketchbook`) "TargetTexture" NewTexture)
  (`MaterialInstanceDynamic.SetScalarParameterValue` (`self.MID_Sketchbook`) "RevealAmount" 0.0)
  (`TimelineComponent.SetPlayRate` (`self.TL_DrawReveal`) RevealPlayRate)
  (bind (_direction _reveal) (`Timeline|TL_DrawReveal` :!via `PlayFromStart` :!label _label)
    (:`Update`
      (`MaterialInstanceDynamic.SetScalarParameterValue` (`self.MID_Sketchbook`) "RevealAmount" _reveal))
    (:`Finished`
      (set `self.CurrentTexture` (`self.PendingTexture`)))))

(event `StopSketchbookReveal`
  (goto _label :!via `Stop`))

(fn `Interact`
  (`parent.Interact`)
  (set `self.CanInteract` false)
  (bind _outactors (`GameplayStatics.GetAllActorsOfClass` "/Game/00_MY/03_BP/BP_Part1Manager.BP_Part1Manager_C"))
  (bind _output (`|GetArrayItem` _outactors))
  (switch `int` (`/Game/00_MY/03_BP/BP_Part1Manager.Part1ChoiceResult` _output)
    (:`0`
      (`self.RevealSketchbookTexture` (`self.Tex_Draft`) 1.0)
      (`/Game/00_MY/03_BP/BP_Part1Manager.StartHomeworkScene` _output))
    (:`1`
      (`self.RevealSketchbookTexture` (`self.Tex_Stable`) 1.0)
      (`/Game/00_MY/03_BP/BP_Part1Manager.Part1_DrawStableResult` _output))
    (:`2`
      (`self.RevealSketchbookTexture` (`self.Tex_Anxious`) 1.0)
      (`/Game/00_MY/03_BP/BP_Part1Manager.Part1_DrawEndureResult` _output))))

(fn `UserConstructionScript`)