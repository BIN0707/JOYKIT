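; Actor that shows an animated inspect object, swapping an animated skeletal mesh for a static result mesh when the inspection completes.
; Setup receives meshes, animation, text, read delay and owner pawn from the caller.
; Play and reset events toggle visibility and control the animation.
; The finish event, not triggered within this graph, reveals the result mesh, tells the owner pawn to show the text and fires a finished callback.
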(event `PlayInspectAnimation`
  (`SceneComponent.SetHiddenInGame` (`self.AnimatedMesh`) false false)
  (`SceneComponent.SetHiddenInGame` (`self.ResultMesh`) true false)
  (`SkeletalMeshComponent.PlayAnimation` (`self.AnimatedMesh`) (`self.InspectAnimation`) false))

(event `ResetInspectAnimation`
  (bind _animatedmesh (`self.AnimatedMesh`))
  (`SkeletalMeshComponent.Stop` _animatedmesh)
  (`SceneComponent.SetHiddenInGame` _animatedmesh false false)
  (`SceneComponent.SetHiddenInGame` (`self.ResultMesh`) true false))

(event `FinishInspectAnimation`
  (bind _ownerpawnref (`self.OwnerPawnRef`))
  (`SceneComponent.SetHiddenInGame` (`self.AnimatedMesh`) true false)
  (`SceneComponent.SetHiddenInGame` (`self.ResultMesh`) false false)
  (`/Engine/EditorBlueprintResources/StandardMacros.IsValid` _ownerpawnref
    (:`Is Valid`
      (`/Game/VRTemplate/Blueprints/VRPawn.ShowAnimatedInspectText` _ownerpawnref (`self.InspectText`) (`self.ReadDelay`))
      (`self.OnInspectAnimationFinished`))))

(event `SetupAnimatedInspect`
  (params (NewInspectText :type Text) (NewReadDelay :type "Float (double-precision)") (NewOwnerPawn :type "/Game/VRTemplate/Blueprints/VRPawn Object Reference") (NewSkeletalMesh :type "SkeletalMesh Object Reference") (NewAnimation :type "AnimSequence Object Reference") (NewResultMesh :type "StaticMesh Object Reference"))
  (set `self.InspectText` NewInspectText)
  (set `self.ReadDelay` NewReadDelay)
  (set `self.OwnerPawnRef` NewOwnerPawn)
  (set `self.InspectSkeletalMesh` NewSkeletalMesh)
  (set `self.InspectAnimation` NewAnimation)
  (set `self.InspectResultMesh` NewResultMesh)
  (`SkeletalMeshComponent.SetSkeletalMeshAsset` (`self.AnimatedMesh`) (`self.InspectSkeletalMesh`))
  (`StaticMeshComponent.SetStaticMesh` (`self.ResultMesh`) (`self.InspectResultMesh`)))

(fn `UserConstructionScript`)