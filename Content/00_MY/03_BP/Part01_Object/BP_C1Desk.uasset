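; BP_C1Desk is an interactable desk that moves the VR pawn into the Part 1 desk scene.
; Interact calls its parent, disables further interaction, then continues only if BP_Part1Manager reports DeskUnlocked.
; It teleports the pawn to DeskTeleportRef's location and rotation, then calls StartDeskScene on the manager.
; The StartDeskSequence event runs the same teleport and scene start without the unlock check.
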(event `StartDeskSequence`
  (bind _deskteleportref (`self.DeskTeleportRef`))
  (bind _asvrpawn (cast `/Game/VRTemplate/Blueprints/VRPawn` (`GameplayStatics.GetPlayerPawn` 0)))
  (`self.K2_SetActorLocationAndRotation` _asvrpawn (`self.K2_GetActorLocation` _deskteleportref) (`self.K2_GetActorRotation` _deskteleportref) false true)
  (bind _outactors (`GameplayStatics.GetAllActorsOfClass` "/Game/00_MY/03_BP/BP_Part1Manager.BP_Part1Manager_C"))
  (`/Game/00_MY/03_BP/BP_Part1Manager.StartDeskScene` (`|GetArrayItem` _outactors)))

(fn `Interact`
  (bind _deskteleportref (`self.DeskTeleportRef`))
  (`parent.Interact`)
  (set `self.CanInteract` false)
  (bind _outactors (`GameplayStatics.GetAllActorsOfClass` "/Game/00_MY/03_BP/BP_Part1Manager.BP_Part1Manager_C"))
  (if (`/Game/00_MY/03_BP/BP_Part1Manager.bDeskUnlocked` (`|GetArrayItem` _outactors))
    (bind _asvrpawn (cast `/Game/VRTemplate/Blueprints/VRPawn` (`GameplayStatics.GetPlayerPawn` 0)))
    (`self.K2_SetActorLocationAndRotation` _asvrpawn (`self.K2_GetActorLocation` _deskteleportref) (`self.K2_GetActorRotation` _deskteleportref) false true)
    (bind _outactors_2 (`GameplayStatics.GetAllActorsOfClass` "/Game/00_MY/03_BP/BP_Part1Manager.BP_Part1Manager_C"))
    (`/Game/00_MY/03_BP/BP_Part1Manager.StartDeskScene` (`|GetArrayItem` _outactors_2))))

(fn `UserConstructionScript`)