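; BP_C1JoyKitBox is an interactable JoyKit box for Part 1 that opens and offers a manual to inspect.
; Interact disables the prompt and plays the one-shot box-opening animation.
; ShowJoyKitManualInspect opens the VR pawn's inspect view with the manual mesh, material and Korean label.
; CompleteInvestigation, guarded to run once, disables interaction and notifies BP_Part1Manager to start the box inspect step.
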(event `ShowJoyKitManualInspect`
  (bind _asvrpawn (cast `/Game/VRTemplate/Blueprints/VRPawn` (`GameplayStatics.GetPlayerPawn` 0)))
  (`/Game/VRTemplate/Blueprints/VRPawn.OpenInspect` _asvrpawn "/Game/00_MY/01_Modeling/Part1_M/JoyKit_Manual.JoyKit_Manual" "/Game/00_MY/04_Texture/Part1/Manual/Manual_M.Manual_M" "JOYKIT 설명서" self))

(event `self.CompleteInvestigation`
  (if (not (`self.HasInteracted`))
    (set `self.HasInteracted` true)
    (set `self.CanInteract` false)
    (`self.UpdatePromptVisibility`)
    (bind _outactors (`GameplayStatics.GetAllActorsOfClass` "/Game/00_MY/03_BP/BP_Part1Manager.BP_Part1Manager_C"))
    (`/Game/00_MY/03_BP/BP_Part1Manager.StartJoyKitBoxInspect` (`|GetArrayItem` _outactors))))

(fn `Interact`
  (set `self.CanInteract` false)
  (`self.UpdatePromptVisibility`)
  (`SkeletalMeshComponent.PlayAnimation` (`self.Joykitbox`) "/Game/00_MY/05_Animation/Box_open_Anim.Box_open_Anim" false))

(fn `UserConstructionScript`)